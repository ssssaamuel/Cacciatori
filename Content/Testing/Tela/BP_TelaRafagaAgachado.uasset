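; Test actor that applies a wind gust, presumably to cloth given its name, while the first-person player is crouched inside a trigger zone.
; Overlap events on Zona track whether the player is inside and cache their capsule component.
; Every Tick, a capsule half-height below a fixed threshold serves as the crouch check, setting Viento's strength to FuerzaViento, otherwise to zero.
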(event OnComponentBeginOverlap(Zona)
  (params (OverlappedComponent :type Primitive%20Component%20Object%20Reference) (OtherActor :type Actor%20Object%20Reference) (OtherComp :type Primitive%20Component%20Object%20Reference) (OtherBodyIndex :type Integer) (bFromSweep :type Boolean) (SweepResult :type Hit%20Result%20Structure%20%28by%20ref%29))
  (bind _asbp_first_person_character (Utilities|Casting|CastToBP_FirstPersonCharacter OtherActor))
  (Variables|Default|SetJugadorDentro true)
  (Variables|Default|SetCapsulaJugador (Variables|/Script/Engine.Character|GetCapsuleComponent _asbp_first_person_character)))

(event OnComponentEndOverlap(Zona)
  (params (OverlappedComponent :type Primitive%20Component%20Object%20Reference) (OtherActor :type Actor%20Object%20Reference) (OtherComp :type Primitive%20Component%20Object%20Reference) (OtherBodyIndex :type Integer))
  (Utilities|Casting|CastToBP_FirstPersonCharacter OtherActor)
  (Variables|Default|SetJugadorDentro false))

(event EventBeginPlay)

(event Collision|EventActorBeginOverlap
  (params (OtherActor :type Actor%20Object%20Reference)))

(event EventTick
  (params (DeltaSeconds :type Float%20%28single-precision%29))
  (if (Variables|Default|GetJugadorDentro)
    (Class|WindDirectionalSourceComponent|SetStrength (Variables|Default|GetViento) (select (< (Components|Capsule|GetScaledCapsuleHalfHeight (Variables|Default|GetCapsulaJugador)) (Math|Float|MakeLiteralFloat 7e+01)) (Variables|Default|GetFuerzaViento) (Math|Float|MakeLiteralFloat 0.0)))
    (else
      (Class|WindDirectionalSourceComponent|SetStrength (Variables|Default|GetViento) 0.0))))

(fn ConstructionScript)